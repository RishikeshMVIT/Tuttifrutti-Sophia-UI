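; BP_Inventory stores the owner's items in a fixed-size slot array and shows them in a WB_Inventory widget, toggled with I.
; E runs a debug-drawn sphere trace below the owner to find a BP_Item.
; One pass over slots stacks it up to the max size or fills an empty slot, whichever comes first.
; Pickup refreshes the widget and destroys the item, whose validity check blocks further inserts.
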(event EventBeginPlay
  (bind _returnvalue (UserInterface|CreateWidget "/Game/Systems/Inventory_Rishi/Widgets/WB_Inventory.WB_Inventory_C"))
  (Variables|Default|SetInventory%20Widget _returnvalue)
  (Utilities|Array|Resize (Variables|Default|GetItems) (Variables|Default|GetInventorySize))
  (Default|LoadInventory (Variables|Default|GetInventory%20Widget) self))

(event Input|KeyboardEvents|I
  (params (Key :type Key%20Structure :default "None"))
  (:Pressed
    (if (Widget|IsVisible (Variables|Default|GetInventory%20Widget))
      (Widget|RemovefromParent (Variables|Default|GetInventory%20Widget))
      (else
        (UserInterface|Viewport|AddtoViewport (Variables|Default|GetInventory%20Widget) 0)))))

(event Input|KeyboardEvents|E
  (params (Key :type Key%20Structure :default "None"))
  (bind _returnvalue (Components|GetOwner))
  (bind _returnvalue_2 (Transformation|GetActorLocation _returnvalue))
  (bind _returnvalue_3 (- _returnvalue_2 "0.000000,0.000000,50.000000"))
  (:Pressed
    (bind _outhit (Collision|SphereTraceByChannel _returnvalue_3 _returnvalue_3 1.5e+02 "TraceTypeQuery4" false 0 "ForDuration"))
    (bind _asbp_item (Utilities|Casting|CastToBP_Item (.HitActor (Collision|BreakHitResult _outhit))))
    (for (_array_element _array_index) (Variables|Default|GetItems)
      (Utilities|IsValid _asbp_item
        (:Is%20Valid
          (if (Math|Boolean|ANDBoolean (Utilities|Enum|Equal(Enum) (.Name (Utilities|Struct|BreakS_ItemDetails _array_element)) (.name (Variables|/Game/Systems/Inventory_Rishi/Blueprints/BP_Item.BP_Item_C|GetItemDetails _asbp_item))) (.isstackable (Variables|/Game/Systems/Inventory_Rishi/Blueprints/BP_Item.BP_Item_C|GetItemDetails _asbp_item)) (<= (+ (.Quantity (Utilities|Struct|BreakS_ItemDetails _array_element)) (.quantity (Variables|/Game/Systems/Inventory_Rishi/Blueprints/BP_Item.BP_Item_C|GetItemDetails _asbp_item))) (Variables|Default|GetMaxStackSize)))
            (Utilities|Array|SetArrayElem (Variables|Default|GetItems) _array_index (Utilities|Struct|MakeS_ItemDetails (.Name (Utilities|Struct|BreakS_ItemDetails (Variables|/Game/Systems/Inventory_Rishi/Blueprints/BP_Item.BP_Item_C|GetItemDetails _asbp_item))) (+ (.Quantity (Utilities|Struct|BreakS_ItemDetails _array_element)) (.quantity (Variables|/Game/Systems/Inventory_Rishi/Blueprints/BP_Item.BP_Item_C|GetItemDetails _asbp_item))) (.Thumbnail (Utilities|Struct|BreakS_ItemDetails (Variables|/Game/Systems/Inventory_Rishi/Blueprints/BP_Item.BP_Item_C|GetItemDetails _asbp_item))) (.Mesh (Utilities|Struct|BreakS_ItemDetails (Variables|/Game/Systems/Inventory_Rishi/Blueprints/BP_Item.BP_Item_C|GetItemDetails _asbp_item))) (.IsStackable (Utilities|Struct|BreakS_ItemDetails (Variables|/Game/Systems/Inventory_Rishi/Blueprints/BP_Item.BP_Item_C|GetItemDetails _asbp_item)))))
            (Default|LoadInventory (Variables|Default|GetInventory%20Widget) self :!label _label)
            (Actor|DestroyActor _asbp_item)
            (elif (== (.Quantity (Utilities|Struct|BreakS_ItemDetails _array_element)) 0)
              (Utilities|Array|SetArrayElem (Variables|Default|GetItems) _array_index (Variables|/Game/Systems/Inventory_Rishi/Blueprints/BP_Item.BP_Item_C|GetItemDetails _asbp_item))
              (goto _label))))))))